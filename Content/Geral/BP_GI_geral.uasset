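; Game Instance that owns the game's save data, held in a BP_SG_geral object.
; On Init it synchronously loads the save slot, or creates a fresh save object in memory if none exists.
; SalvarJogador copies player info into that object and writes it to the slot, while PegarDadosSalvos exposes the data.
; Save and load events take an Async flag to choose background or blocking operation.
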(event `self.ReceiveInit`
  ;[1 1 1] Carrega o jogo quando essa blueprint inicia
  (`self.CarregarJogo` false))

(event `self.SalvarJogo`
  (params (async :type Boolean))
  ;[1 1 1] Salvar jogo
  (if async
    (`AsyncActionHandleSaveGame.AsyncSaveGameToSlot` (`self.dadosSalvos`) (`self.jogoSalvo`))
    (else
      (`GameplayStatics.SaveGameToSlot` (`self.dadosSalvos`) (`self.jogoSalvo`)))))

(event `self.CarregarJogo`
  (params (async :type Boolean))
  ;[1 1 1] Carregar jogo salvo
  (bind _returnvalue (`GameplayStatics.DoesSaveGameExist` (`self.jogoSalvo`)))
  (if _returnvalue
    (if async
      ;;[1 1 1] Carrega o jogo em segundo plano, o jogador pode jogar enquanto o jogo carrega
      (bind _savegame (`AsyncActionHandleSaveGame.AsyncLoadGameFromSlot` (`self.jogoSalvo`))
        (:`Completed`
          (bind _asbp_sg_geral (cast `/Game/Geral/BP_SG_geral` _savegame))
          (set `self.dadosSalvos` _asbp_sg_geral)))
      (else
        ;;[1 1 1] Carrega o jogo e depois da o controle para o jogador, usado para quando não tem muita coisa para carregar
        (bind _returnvalue_2 (`GameplayStatics.LoadGameFromSlot` (`self.jogoSalvo`)))
        (bind _asbp_sg_geral_2 (cast `/Game/Geral/BP_SG_geral` _returnvalue_2))
        (set `self.dadosSalvos` _asbp_sg_geral_2)))
    (else
      (bind _returnvalue_3 (`GameplayStatics.CreateSaveGameObject` "/Game/Geral/BP_SG_geral.BP_SG_geral_C"))
      (set `self.dadosSalvos` _returnvalue_3))))

(event `self.SalvarJogador`
  (params (infoJogador :type "/Game/Geral/ST_infoJogador Structure") (async :type Boolean))
  (set `/Game/Geral/BP_SG_geral.sg_infoJogador` infoJogador (`self.dadosSalvos`))
  (`self.SalvarJogo` async))

(fn `PegarDadosSalvos`
  (returns (dadosSalvos :type "/Game/Geral/BP_SG_geral Object Reference"))
  (return (`self.dadosSalvos`)))