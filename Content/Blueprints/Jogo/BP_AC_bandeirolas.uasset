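; Bunting ("bandeirolas") actor that hangs a spline mesh between the "Top" sockets of two static meshes.
; The construction script caches both meshes, and each LiveLinkComponentController update calls Update to move the spline's endpoints to those sockets.
; Tangents get only a Z value, from half the height difference offset oppositely by distance times GravityPull, to fake a gravity sag.
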(event `self.LiveLinkComponentController.OnLiveLinkUpdated`
  (params (DeltaTime :type "Float (single-precision)"))
  (`self.Update`))

(fn `Update`
  (bind _returnvalue_location (`KismetMathLibrary.BreakTransform` (`SceneComponent.GetSocketTransform` (`self.VEnd Mesh`) "Top" "RTS_Actor")))
  (bind _returnvalue_location_2 (`KismetMathLibrary.BreakTransform` (`SceneComponent.GetSocketTransform` (`self.VStart Mesh`) "Top" "RTS_Actor")))
  (bind _returnvalue (`KismetMathLibrary.MakeVector` (.x _returnvalue_location) (.y _returnvalue_location) (.z _returnvalue_location)))
  (bind _returnvalue_2 (`KismetMathLibrary.MakeVector` (.x _returnvalue_location_2) (.y _returnvalue_location_2) (.z _returnvalue_location_2)))
  (bind _returnvalue_3 (- _returnvalue_2 _returnvalue))
  (bind _returnvalue_4 (- _returnvalue_2 _returnvalue))
  (bind _returnvalue_5 (`KismetMathLibrary.VSize` _returnvalue_3))
  (bind _returnvalue_6 (`KismetMathLibrary.VSize` _returnvalue_4))
  (`SplineMeshComponent.SetStartPosition` (`self.SplineMesh`) _returnvalue_2 true)
  (`SplineMeshComponent.SetEndPosition` (`self.SplineMesh`) _returnvalue true)
  (`SplineMeshComponent.SetStartTangent` (`self.SplineMesh`) (`KismetMathLibrary.MakeVector` 0.0 0.0 (- (.z (* (* (`KismetMathLibrary.Normal` _returnvalue_4) _returnvalue_6) 0.5)) (* _returnvalue_6 (`self.GravityPull`)))) true)
  (`SplineMeshComponent.SetEndTangent` (`self.SplineMesh`) (`KismetMathLibrary.MakeVector` 0.0 0.0 (+ (.z (* (* (`KismetMathLibrary.Normal` _returnvalue_3) _returnvalue_5) 0.5)) (* _returnvalue_5 (`self.GravityPull`)))) true))

(fn `UserConstructionScript`
  (set `self.VStart Mesh` (`self.StaticMesh`))
  (set `self.VEnd Mesh` (`self.StaticMesh1`)))