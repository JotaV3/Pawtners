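; Void trigger box that returns players who fall into it to their checkpoint.
; On the server, an overlap by BP_CH_jogador sends a TeleportarJogador message to the Game Mode with that player and their stored checkpoint location.
; The construction script scales the collision component from the Largura, Comprimento and Altura variables (width, length, height), so each instance can be sized separately.
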(event `self.CollisionComponent.OnComponentBeginOverlap`
  (params (OverlappedComponent :type "PrimitiveComponent Object Reference") (OtherActor :type "Actor Object Reference") (OtherComp :type "PrimitiveComponent Object Reference") (OtherBodyIndex :type Integer) (bFromSweep :type Boolean) (SweepResult :type "HitResult Structure (by ref)"))
  ;[1 1 1] Envia um sinal para quando o jogador cair no void
  (if (`KismetSystemLibrary.IsServer`)
    (bind _asbp_ch_jogador (cast `/Game/Personagens/Content/BP_CH_jogador` OtherActor))
    (bind _checkpoint_location (`KismetMathLibrary.BreakTransform` (`/Game/Personagens/Content/BP_CH_jogador.checkpoint` _asbp_ch_jogador)))
    (message `/Game/Blueprints/Jogo/BPI_teleportarJogador.TeleportarJogador` (`GameplayStatics.GetGameMode`) _asbp_ch_jogador _checkpoint_location)))

(fn `UserConstructionScript`
  (`SceneComponent.SetWorldScale3D` (`self.CollisionComponent`) (`KismetMathLibrary.MakeVector` (`self.largura`) (`self.comprimento`) (`self.altura`))))