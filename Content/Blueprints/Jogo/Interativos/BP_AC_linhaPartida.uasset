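; Starting-line actor that creates player start points (BP_PS_jogo) for a network session.
; SE_ConfigurarSpawners stores the session's connection count, then spawns one start 400 units along X from the Spawner component and prints debug locations.
; CalcularPosicaoSpawner alternates sides on Y with a widening offset, but the spawn transform does not use it.
; BeginPlay is empty, and the authority check and setup call are disconnected.
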(event `self.ReceiveBeginPlay`)

(event `SE_ConfigurarSpawners`
  (bind _returnvalue (`SceneComponent.K2_GetComponentToWorld` (`self.spawner`)))
  (bind _numconnections (`AdvancedSessionsLibrary.GetSessionSettings`)
    (:`OnSuccess`
      (set `self.qtd_maxJogadores` _numconnections)
      (for _ (range 1)
        (`self.CalcularPosicaoSpawner`)
        (bind _returnvalue_2 (`|SpawnActorFromClass` "/Game/Blueprints/Jogo/BP_PS_jogo.BP_PS_jogo_C" (`KismetMathLibrary.MakeTransform` (`KismetMathLibrary.MakeVector` (+ (.x (.location _returnvalue)) 400.0) (.y (.location _returnvalue)) (.z (.location _returnvalue))) (.rotation _returnvalue) (1.0 1.0 1.0)) "Undefined" "OverrideRootScale" null null))
        (`KismetSystemLibrary.PrintString` (`KismetStringLibrary.Conv_VectorToString` (`self.K2_GetActorLocation` _returnvalue_2)) true true (struct :`G` 0.66 :`B` 1.0 :`A` 1.0) 20.0)
        (`KismetSystemLibrary.PrintString` (`KismetStringLibrary.Conv_VectorToString` (`SceneComponent.K2_GetComponentLocation` (`self.spawner`))) true true (struct :`R` 1.0 :`G` 0.041135 :`A` 1.0) 20.0)))))

(fn `CalcularPosicaoSpawner`
  (returns (localizacao :type "Float (double-precision)"))
  ;[1 1 1] A cada chamada da função a variável "multiplicaY" alterna de 1.0 para -1.0 (uma hora para a direita outra para a esquerda)
  (bind _output_get (set `self.multiplicaY` (* (`self.multiplicaY`) -1.0)))
  ;[1 1 1] A varíavel "razaoLocalizacaoY" determina o quão distante a localização, no eixo Y, do ponto de spawn do jogador(Player Start) estará em relação ao ponto de spawn do servidor(eixoY=0)
  (bind _output_get_2 (set `self.localizacaoY` (* _output_get (`self.razaoLocalizacaoY`))))
  ;[1 1 1] Caso a localização seja negativa, está na hora de fazer um ponto de spawn do outro lado.
  (if (< _output_get_2 0.0)
    (bind _output_get_3 (set `self.razaoLocalizacaoY` (+ (`self.razaoLocalizacaoY`) 400.0)))
    (return _output_get_3)))

(fn `UserConstructionScript`)