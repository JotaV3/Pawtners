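; Interactive platform actor that slides back and forth continuously along its local X axis.
; BeginPlay starts a server-style Mover timeline that offsets the Plataforma component by the curve value scaled by Direcao and Distancia.
; When the timeline finishes, the Reverse macro toggles a flag to alternate between playing and reversing it, creating an endless ping-pong motion.
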(event `self.ReceiveBeginPlay`
  (`self.SR_Mover`))

(event `SR_Mover`
  (bind (_direction _mover) (`Timeline|mover` :!label _label)
    (:`Update`
      (`SceneComponent.K2_SetRelativeLocation` (`self.plataforma`) (`KismetMathLibrary.MakeVector` (/ (* (.x _mover) (`self.direcao`)) (`self.distancia`))) false false))
    (:`Finished`
      (`self.Reverse`
        (:`iniciar`
          (goto _label))
        (:`reverter`
          (goto _label :!via `Reverse`))))))

(fn `UserConstructionScript`)