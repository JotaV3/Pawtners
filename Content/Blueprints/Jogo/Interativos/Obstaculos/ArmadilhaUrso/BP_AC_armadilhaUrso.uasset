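; Bear trap obstacle actor that catches a player who steps into its sphere.
; On overlap, SR_PrenderJogador disables the character's movement and has the game mode teleport them to the sphere's center.
; For a locally controlled player, it also enables key pressing on the character, passing the trap's key-press widget; release logic lives outside this Blueprint.
; The construction script scales the trap from Escala.
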(event `self.ReceiveBeginPlay`
  (bind _aswb_pressionar_tecla (cast `/Game/Blueprints/Jogo/Interativos/Obstaculos/ArmadilhaUrso/WB_pressionarTecla` (`WidgetComponent.GetWidget` (`self.Widget`))))
  (set `self.As WB Pressionar Tecla` _aswb_pressionar_tecla))

(event `SR_PrenderJogador`
  ;[1 1 1] Prende o jogador na armadilha de urso / desabilita os movimentos do jogador e teleporta ele para o centro da armadilha
  (`CharacterMovementComponent.DisableMovement` (`Character.CharacterMovement` (`self.As BP CH Jogador`)))
  (message `/Game/Blueprints/Jogo/BPI_teleportarJogador.TeleportarJogador` (`GameplayStatics.GetGameMode`) null (`self.LocalArmadilha`)))

(event `self.Sphere.OnComponentBeginOverlap`
  (params (OverlappedComponent :type "PrimitiveComponent Object Reference") (OtherActor :type "Actor Object Reference") (OtherComp :type "PrimitiveComponent Object Reference") (OtherBodyIndex :type Integer) (bFromSweep :type Boolean) (SweepResult :type "HitResult Structure (by ref)"))
  ;[1 1 1] Verifica qual jogador encostou na armadilha de urso
  (`|ExecutionSequence`
    (:`then_0`
      (bind _asbp_ch_jogador (cast `/Game/Personagens/Content/BP_CH_jogador` OtherActor))
      (set `self.As BP CH Jogador` _asbp_ch_jogador)
      (`self.SR_PrenderJogador`)
      (if (`Pawn.IsLocallyControlled` (`self.As BP CH Jogador`))
        (`/Game/Personagens/Content/BP_CH_jogador.LiberarPressionamentoTecla` (`self.As BP CH Jogador`) (`self.As WB Pressionar Tecla`) true)))))

(fn `LocalArmadilha`
  (returns (local :type "Vector Structure"))
  ;[1 1 1] Retorna o local exato do centro da armadilha
  (return (`SceneComponent.K2_GetComponentLocation` (`self.Sphere`))))

(fn `UserConstructionScript`
  (bind _escala (`self.escala`))
  (`SceneComponent.SetWorldScale3D` (`self.armadilhaUrso`) (`KismetMathLibrary.MakeVector` _escala _escala _escala)))