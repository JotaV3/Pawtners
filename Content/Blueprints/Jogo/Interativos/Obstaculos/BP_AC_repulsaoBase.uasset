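; Base repulsion obstacle that knocks the player away when BP_CH_jogador hits its mesh, with optional self-destruction after a hit.
; On hit, an SR event calls the player's air-control event, removing control in the air, then launches the character with full velocity override.
; Launch direction is the flattened mesh-to-player vector tilted 20 degrees upward, scaled by VelocidadeLancamento.
; A DoOnce with delayed reset debounces hits, and the construction script uniformly scales the mesh.
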(event `SR_LancarJogador`
  (params (jogador :type "/Game/Personagens/Content/BP_CH_jogador Object Reference"))
  ;[1 1 1] Tira o controle no ar do jogador e lança ele a uma distância definida pela variável "velocidadeLancamento"
  (`/Game/Personagens/Content/BP_CH_jogador.SR_ControleAereo` jogador)
  (`Character.LaunchCharacter` jogador (`self.LancarJogador` jogador) true true))

(event `self.malha.OnComponentHit`
  (params (HitComponent :type "PrimitiveComponent Object Reference") (OtherActor :type "Actor Object Reference") (OtherComp :type "PrimitiveComponent Object Reference") (NormalImpulse :type "Vector Structure") (Hit :type "HitResult Structure (by ref)"))
  (`/Engine/EditorBlueprintResources/StandardMacros.DoOnce` false :!label _label
    (:`Completed`
      (`|ExecutionSequence`
        (:`then_0`
          (`|ExecutionSequence`
            (:`then_0`
              (bind _asbp_ch_jogador (cast `/Game/Personagens/Content/BP_CH_jogador` OtherActor))
              (`self.SR_LancarJogador` _asbp_ch_jogador))
            (:`then_1`
              (if (`self.destruirAtor`)
                (`self.K2_DestroyActor`)))))
        (:`then_1`
          (`KismetSystemLibrary.Delay` 0.3)
          (goto _label :!via `Reset`))))))

(fn `LancarJogador`
  (params (jogador :type "Actor Object Reference"))
  (returns (ReturnValue :type "Vector Structure"))
  (bind _returnvalue (`self.K2_GetActorLocation` jogador))
  (bind _returnvalue_2 (`SceneComponent.K2_GetComponentLocation` (`self.malha`)))
  (return (* (`KismetMathLibrary.Normal` (`KismetMathLibrary.RotateAngleAxis` (`KismetMathLibrary.ProjectVectorOnToPlane` (`KismetMathLibrary.GetDirectionUnitVector` _returnvalue_2 _returnvalue) (0.0 0.0 1.0)) -20.0 (`KismetMathLibrary.GetRightVector` (`KismetMathLibrary.FindLookAtRotation` _returnvalue_2 _returnvalue)))) (`self.velocidadeLancamento`))))

(fn `UserConstructionScript`
  (bind _escala (`self.escala`))
  (`SceneComponent.SetWorldScale3D` (`self.malha`) (`KismetMathLibrary.MakeVector` _escala _escala _escala)))