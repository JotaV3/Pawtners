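; BP_AC_empurrador is a pusher obstacle that slides back and forth and knocks players away.
; From BeginPlay, it loops the Empurrar timeline, using the Reverter flip-flop macro to alternate extending and retracting, with a short random delay between cycles.
; Colisao overlaps with BP_CH_jogador trigger SR_LancarJogador, launching the player along the collider's flattened forward vector, tilted slightly and scaled by VelocidadeLancamento.
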(event `self.ReceiveBeginPlay`
  (`self.SR_Empurrar`))

(event `SR_Empurrar`
  ;[1 1 1] O tempo de para empurrar é um número aletório
  (`KismetSystemLibrary.Delay` (`KismetMathLibrary.RandomFloatInRange` 0.5 1.0) :!label _label)
  ;[1 1 1] Faz o movimento de ir para frente e para trás
  (bind (_direction _empurra) (`Timeline|Empurrar` :!label _label_2)
    (:`Update`
      (`SceneComponent.K2_SetRelativeLocation` (`self.empurrador`) _empurra false false))
    (:`Finished`
      (`self.Reverter`
        (:`Iniciar`
          (goto _label))
        (:`Reverter`
          (goto _label_2 :!via `Reverse`))))))

(event `SR_LancarJogador`
  (params (jogador :type "/Game/Personagens/Content/BP_CH_jogador Object Reference"))
  (bind _colisao (`self.colisao`))
  (`Character.LaunchCharacter` jogador (* (`KismetMathLibrary.Normal` (`KismetMathLibrary.RotateAngleAxis` (`KismetMathLibrary.ProjectVectorOnToPlane` (`SceneComponent.GetForwardVector` _colisao) (0.0 0.0 1.0)) -10.0 (`KismetMathLibrary.GetRightVector` (`KismetMathLibrary.FindLookAtRotation` (`SceneComponent.K2_GetComponentLocation` _colisao) (`self.K2_GetActorLocation` (stale `self.colisao.OnComponentBeginOverlap` _asbp_ch_jogador)))))) (`self.velocidadeLancamento`)) true false))

(event `self.colisao.OnComponentBeginOverlap`
  (params (OverlappedComponent :type "PrimitiveComponent Object Reference") (OtherActor :type "Actor Object Reference") (OtherComp :type "PrimitiveComponent Object Reference") (OtherBodyIndex :type Integer) (bFromSweep :type Boolean) (SweepResult :type "HitResult Structure (by ref)"))
  (bind _asbp_ch_jogador (cast `/Game/Personagens/Content/BP_CH_jogador` OtherActor))
  (`self.SR_LancarJogador` _asbp_ch_jogador))

(fn `UserConstructionScript`)