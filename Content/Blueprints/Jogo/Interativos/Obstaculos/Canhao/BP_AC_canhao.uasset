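; BP_AC_canhao is a cannon obstacle that repeatedly fires snowballs from its Arrow component.
; BeginPlay starts SR_AtivarCanhao, an endless loop that waits a random Min–Max delay before each shot.
; Each shot spawns a BPChild_AC_bolaNeve, sets its lifespan, DestruirAtor value and mesh scale from cannon variables.
; It launches the mesh with a velocity-change impulse along the arrow's forward vector with Z zeroed, scaled by VelocidadeProjetil.
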(event `self.ReceiveBeginPlay`
  (`self.SR_AtivarCanhao`))

(event `SR_AtivarCanhao`
  (bind _escalabolaneve (`self.escalaBolaNeve`))
  (bind (_returnvalue_x _returnvalue_y) (`KismetMathLibrary.BreakVector` (`SceneComponent.GetForwardVector` (`self.Arrow`))))
  (`KismetSystemLibrary.Delay` (`KismetMathLibrary.RandomFloatInRange` (`self.Min`) (`self.Max`)) :!label _label)
  (bind _returnvalue (`|SpawnActorFromClass` "/Game/Blueprints/Jogo/Interativos/Obstaculos/Canhao/BPChild_AC_bolaNeve.BPChild_AC_bolaNeve_C" (`SceneComponent.K2_GetComponentToWorld` (`self.Arrow`)) "Undefined" "OverrideRootScale" null null))
  (`self.SetLifeSpan` _returnvalue (`self.Lifespan_bolaNeve`))
  (set `/Game/Blueprints/Jogo/Interativos/Obstaculos/BP_AC_repulsaoBase.destruirAtor` (`self.destruirBolaNeve`) _returnvalue)
  (bind _malha (`/Game/Blueprints/Jogo/Interativos/Obstaculos/BP_AC_repulsaoBase.malha` _returnvalue))
  (`SceneComponent.SetWorldScale3D` _malha (`KismetMathLibrary.MakeVector` _escalabolaneve _escalabolaneve _escalabolaneve))
  (`PrimitiveComponent.AddImpulse` _malha (* (`KismetMathLibrary.MakeVector` _returnvalue_x _returnvalue_y) (`self.velocidadeProjetil`)) "None" true)
  (goto _label))

(fn `UserConstructionScript`)