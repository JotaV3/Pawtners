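; BP_AC_varredor is a sweeper obstacle that spins around Z and knocks players away on contact.
; From BeginPlay, the Girar timeline drives the Pivo yaw, with Direcao as multiplier, while the construction script applies Escala to the Varredor.
; Hits on BP_CH_jogador call the player's SRControleAereo, then LaunchCharacter away from the impact point at VelocidadeLancamento.
; A DoOnce with delayed reset debounces repeated hits.
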(event `self.ReceiveBeginPlay`
  (`self.SR_Girar`))

(event `SR_Girar`
  ;[1 1 1] Gira o objeto no eixo Z. Variável "velocidade" define o quão rápido o objeto vai girar
  (bind (_direction _girareixoz) (`Timeline|Girar`)
    (:`Update`
      (`SceneComponent.K2_SetRelativeRotation` (`self.pivo`) (`KismetMathLibrary.MakeRotator` 0.0 0.0 (* (.z _girareixoz) (`self.direcao`))) false false))))

(event `self.varredor.OnComponentHit`
  (params (HitComponent :type "PrimitiveComponent Object Reference") (OtherActor :type "Actor Object Reference") (OtherComp :type "PrimitiveComponent Object Reference") (NormalImpulse :type "Vector Structure") (Hit :type "HitResult Structure (by ref)"))
  ;[1 1 1] Knockback
  (`/Engine/EditorBlueprintResources/StandardMacros.DoOnce` false :!label _label
    (:`Completed`
      (`|ExecutionSequence`
        (:`then_0`
          (bind _asbp_ch_jogador (cast `/Game/Personagens/Content/BP_CH_jogador` OtherActor))
          (`self.SR_LancarJogador` _asbp_ch_jogador))
        (:`then_1`
          (`KismetSystemLibrary.Delay` 0.3)
          (goto _label :!via `Reset`))))))

(event `SR_LancarJogador`
  (params (jogador :type "/Game/Personagens/Content/BP_CH_jogador Object Reference"))
  ;[1 1 1] Knockback
  (`/Game/Personagens/Content/BP_CH_jogador.SR_ControleAereo` jogador)
  (`Character.LaunchCharacter` jogador (`self.LancarJogador` jogador (`.ImpactPoint` (`GameplayStatics.BreakHitResult` (stale `self.varredor.OnComponentHit` Hit)))) true true))

(fn `LancarJogador`
  (params (jogador :type "Actor Object Reference") (pontoImpacto :type "Vector Structure"))
  (returns (ReturnValue :type "Vector Structure"))
  (return (* (`KismetMathLibrary.Normal` (`KismetMathLibrary.GetDirectionUnitVector` pontoImpacto (`self.K2_GetActorLocation` jogador))) (`self.velocidadeLancamento`))))

(fn `UserConstructionScript`
  (bind _escala (`self.escala`))
  (`SceneComponent.SetWorldScale3D` (`self.varredor`) (`KismetMathLibrary.MakeVector` _escala _escala _escala)))