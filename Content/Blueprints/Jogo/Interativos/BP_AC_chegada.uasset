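; BP_AC_chegada is the finish-line actor that ends the match on the first overlap with its Colisao collision.
; A DoOnce gate starts two branches: for a BP_CH_jogador, the locally controlled player gets the victory widget and sound, while others hear the defeat sound.
; The second branch runs for any overlapping actor: where BP_GM_jogo is available, it stops the music, waits briefly, clears widgets and returns to the lobby.
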(event `self.colisao.OnComponentBeginOverlap`
  (params (OverlappedComponent :type "PrimitiveComponent Object Reference") (OtherActor :type "Actor Object Reference") (OtherComp :type "PrimitiveComponent Object Reference") (OtherBodyIndex :type Integer) (bFromSweep :type Boolean) (SweepResult :type "HitResult Structure (by ref)"))
  (bind _returnvalue (`GameplayStatics.GetPlayerController` 0))
  (`/Engine/EditorBlueprintResources/StandardMacros.DoOnce` false
    (:`Completed`
      (`|ExecutionSequence`
        (:`then_0`
          (bind _asbp_ch_jogador (cast `/Game/Personagens/Content/BP_CH_jogador` OtherActor))
          (if (`Pawn.IsLocallyControlled` _asbp_ch_jogador)
            (bind _returnvalue_2 (`|CreateWidget` "/Game/Interface/Jogo/WB_vitoria.WB_vitoria_C" _returnvalue))
            (`UserWidget.AddToPlayerScreen` _returnvalue_2 0)
            (`GameplayStatics.PlaySound2D` "/Game/Blueprints/Jogo/Som/SW_vitoria.SW_vitoria" 1.0 1.0 0.0 null _returnvalue)
            (else
              (`GameplayStatics.PlaySound2D` "/Game/Blueprints/Jogo/Som/SW_derrota.SW_derrota" 1.0 1.0 0.0 null null))))
        (:`then_1`
          (bind _asbp_gm_jogo (cast `/Game/Blueprints/Jogo/BP_GM_jogo` (`GameplayStatics.GetGameMode`)))
          (`/Game/Blueprints/Jogo/BP_GM_jogo.PararMusica` _asbp_gm_jogo)
          (`KismetSystemLibrary.Delay` 4.0)
          (`WidgetLayoutLibrary.RemoveAllWidgets`)
          (`/Game/Blueprints/Jogo/BP_GM_jogo.VoltarLobby` _asbp_gm_jogo))))))

(fn `UserConstructionScript`)