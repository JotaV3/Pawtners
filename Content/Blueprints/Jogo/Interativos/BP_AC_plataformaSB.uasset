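; BP_AC_plataformaSB is an interactive moving platform that travels up and down continuously from the start of play.
; BeginPlay calls the SR_Mover event, whose Mover timeline sets the Plataforma component's relative Z location from the curve value scaled by Direcao.
; When the timeline finishes, a Reverse macro toggles a boolean to alternate between playing forward and reversing, forming an endless ping-pong loop.
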(event `self.ReceiveBeginPlay`
  (`self.SR_Mover`))

(event `SR_Mover`
  (bind (_direction _mover) (`Timeline|Mover` :!label _label)
    (:`Update`
      (`SceneComponent.K2_SetRelativeLocation` (`self.plataforma`) (`KismetMathLibrary.MakeVector` 0.0 0.0 (* (.z _mover) (`self.direcao`))) false false))
    (:`Finished`
      (`self.Reverse`
        (:`iniciar`
          (goto _label))
        (:`reverter`
          (goto _label :!via `Reverse`))))))

(fn `UserConstructionScript`)