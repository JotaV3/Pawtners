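; Player controller for the race game that handles per-player UI, race music and leaving a match.
; On local start it clears all widgets, and Escape toggles a lazily created in-game menu, switching input mode and cursor.
; Events show the countdown widget, start or stop race music, and destroy the session before returning to the main menu level.
; SE_EnviarServidor, intended to report fallen players to the server, only casts the game mode.
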(event `self.ReceiveBeginPlay`
  (if (`self.IsLocalPlayerController`)
    (`WidgetLayoutLibrary.RemoveAllWidgets`)))

(event `DeixarPartida`
  ;[1 0.5678 0.518] Função para quando o jogador a deixar partida. Destroy a sessão e volta para o menu principal
  (`DestroySessionCallbackProxy.DestroySession` self
    (:`OnSuccess`
      (`GameplayStatics.OpenLevel` "LVL_menuPrincipal"))))

(event `SE_EnviarServidor`
  (params (controleJogador :type "PlayerController Object Reference"))
  ;[1 1 1] Envia o player controller referente ao jogador que caiu do mapa, para o servidor
  (cast `/Game/Blueprints/Jogo/BP_GM_jogo` (`GameplayStatics.GetGameMode`)))

(event `Key|Escape`
  (params (Key :type "Key Structure"))
  ;[1 1 1] Tecla congurada para abrir/fechar o menu do jogo
  (:`Pressed`
    (`/Engine/EditorBlueprintResources/StandardMacros.FlipFlop`
      (:`A`
        (`/Engine/EditorBlueprintResources/StandardMacros.IsValid` (`self.ref_wb_menuJogo`)
          (:`Is Valid`
            _)
          (:`Is Not Valid`
            (bind _returnvalue (`|CreateWidget` "/Game/Interface/Jogo/Menu/WB_menuJogo.WB_menuJogo_C" self))
            (bind _output_get (set `self.ref_wb_menuJogo` _returnvalue))))
        (`UserWidget.AddToViewport` _output_get 0)
        (`WidgetBlueprintLibrary.SetInputMode_GameAndUIEx` self null)
        (set `self.bShowMouseCursor` true))
      (:`B`
        (`Widget.RemoveFromParent` (`self.ref_wb_menuJogo`))
        (`WidgetBlueprintLibrary.SetInputMode_GameOnly` self)
        (set `self.bShowMouseCursor` false)))))

(event `ContagemRegressiva`
  ;[1 1 1] Configurações da corrida
  (bind _returnvalue (`|CreateWidget` "/Game/Interface/Jogo/ContagemRegressiva/WB_contagemRegressiva.WB_contagemRegressiva_C" self))
  (`UserWidget.AddToViewport` _returnvalue 0))

(event `PararMusicaCorrida`
  ;[1 1 1] Configurações da corrida
  (`AudioComponent.FadeOut` (`self.ref_musicaCorrida`) 0.0 0.0 "Linear"))

(event `TocarMusicaCorrida`
  ;[1 1 1] Configurações da corrida
  (bind _returnvalue (`GameplayStatics.SpawnSound2D` "/Game/Blueprints/Jogo/Som/SC_corrida.SC_corrida" 1.0 1.0 0.0 null false false))
  (set `self.ref_musicaCorrida` _returnvalue))

(fn `UserConstructionScript`)