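; Game mode for a multiplayer race that gathers players arriving from the lobby and starts the match countdown.
; Swapped-in controllers are stored in an array, and their pawns are teleported to BP_PS_jogo actors by join index.
; It polls until the session's player count is met, or after several retries starts with more than one player, otherwise server-travelling back.
; It also removes leavers and broadcasts music stop and match exit to controllers.
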(event `self.ReceiveBeginPlay`
  (bind _numconnections (`AdvancedSessionsLibrary.GetSessionSettings`)
    (:`OnSuccess`
      (set `self.qtd_maxJogadores` _numconnections)
      (`self.SituacaoJogadores` 5
        (:`Disponiveis`
          (bind _array_element (`self.Ref_controleJogadores`)
            (:`LoopBody`
              (`/Game/Blueprints/Jogo/BP_PC_jogo.ContagemRegressiva` _array_element))))
        (:`Indisponiveis`
          (`self.VoltarLobby`))))))

(event `self.K2_OnSwapPlayerControllers`
  (params (OldPC :type "PlayerController Object Reference") (NewPC :type "PlayerController Object Reference"))
  ;[1 1 1] Armazena o controle dos jogadores que estavam no lobby para um array
  (bind _asbp_pc_jogo (cast `/Game/Blueprints/Jogo/BP_PC_jogo` NewPC))
  (bind _returnvalue (`KismetArrayLibrary.Array_Add` (`self.controleJogadores`) _asbp_pc_jogo))
  (set `self.IDJogador` _returnvalue)
  (`self.EnfileirarJogadores` _asbp_pc_jogo))

(event `self.TeleportarJogador`
  (params (jogador :type "Actor Object Reference") (local :type "Vector Structure"))
  ;[1 1 1] Teleporta o jogador para o local especifico
  (`self.K2_SetActorLocation` jogador local false true))

(event `self.K2_OnLogout`
  (params (ExitingController :type "Controller Object Reference"))
  ;[1 1 1] Quando um jogador sai da sessão o controle de jogador dele é removido do servidor
  (bind _asbp_pc_jogo (cast `/Game/Blueprints/Jogo/BP_PC_jogo` ExitingController))
  (`KismetArrayLibrary.Array_RemoveItem` (`self.controleJogadores`) _asbp_pc_jogo))

(fn `DestruirSessao`
  (bind (_arrayindex _arrayelement) (`/Engine/EditorBlueprintResources/StandardMacros.ReverseForEachLoop` (`self.controleJogadores`))
    (:`LoopBody`
      (`/Game/Blueprints/Jogo/BP_PC_jogo.DeixarPartida` _arrayelement))))

(fn `EnfileirarJogadores`
  (params (jogador :type "PlayerController Object Reference"))
  (bind _outactors (`GameplayStatics.GetAllActorsOfClass` "/Game/Blueprints/Jogo/BP_PS_jogo.BP_PS_jogo_C"))
  (`self.TeleportarJogador` self (`Controller.K2_GetPawn` jogador) (`self.K2_GetActorLocation` (`|GetArrayItem` _outactors (`self.IDJogador`)))))

(fn `PararMusica`
  (bind _array_element (`self.Ref_controleJogadores`)
    (:`LoopBody`
      (`/Game/Blueprints/Jogo/BP_PC_jogo.PararMusicaCorrida` _array_element))))

(fn `UserConstructionScript`)

(fn `VoltarLobby`
  (locals (nomeLevel :type String :default "LVL_lobby"))
  (`KismetSystemLibrary.ExecuteConsoleCommand` (`KismetStringLibrary.Concat_StrStr` "servertravel " (`local.nomeLevel`)) null))