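; Lobby player controller that manages each player's lobby widget and exchanges player info with the server.
; It fetches saved player info and hands it to BP_GM_lobby for storage.
; Received player arrays rebuild the WB_lobby player list, creating the UI-only widget on first update.
; It also toggles the start-match button by readiness and destroys the session to return to the main menu.
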(event `AdicionarInterfaceLobby`
  ;[1 1 1] Adiciona a interface do lobby
  (bind _returnvalue (`|CreateWidget` "/Game/Interface/Lobby/WB_lobby.WB_lobby_C" self))
  (bind _output_get (set `self.ref_wb_lobby` _returnvalue))
  (`UserWidget.AddToViewport` _output_get 0)
  (`WidgetBlueprintLibrary.SetInputMode_UIOnlyEx` self (`self.ref_wb_lobby`)))

(event `AtualizarInfoJogador`
  ;[1 1 1] Pega as informações salvas do jogador e retorna para o servidor
  (bind _infojogador (`/Game/Blueprints/Biblioteca/Funcoes/BP_FL_geral.InfoJogador`))
  (bind _output_get (set `self.infoJogador` _infojogador))
  (`self.EnviarInfoServidor` _output_get) ; Chama nesta blueprint
)

(event `AtualizarInfoJogadores`
  (params (infoJogador :type "Array of /Game/Geral/ST_infoJogador Structure"))
  (bind _infojogadores (`self.infoJogadores`))
  ;[1 1 1] Atualiza as informações dos jogadores e armazena em um array em cada cliente e cria a interface da lobby e adiciona na tela
  (set `self.infoJogadores` infoJogador)
  (`/Engine/EditorBlueprintResources/StandardMacros.IsValid` (`self.ref_wb_lobby`)
    (:`Is Valid`
      _)
    (:`Is Not Valid`
      (`self.AdicionarInterfaceLobby`) ; Chama nesta blueprint
    ))
  (`PanelWidget.ClearChildren` (`/Game/Interface/Lobby/WB_lobby.vb_listaJogadores` (`self.ref_wb_lobby`)))
  (for _array_element _infojogadores
    (`/Game/Interface/Lobby/WB_lobby.AtualizarListaJogadores` (`self.ref_wb_lobby`) (`KismetArrayLibrary.Array_Length` _infojogadores) _array_element)))

(event `EnviarInfoServidor`
  (params (infoJogador :type "/Game/Geral/ST_infoJogador Structure"))
  ;[1 1 1] Envia as informações para serem manipuladas pelo servidor
  (set `self.infoJogador` infoJogador)
  (bind _asbp_gm_lobby (cast `/Game/Blueprints/Lobby/BP_GM_lobby` (`GameplayStatics.GetGameMode`)))
  (`/Game/Blueprints/Lobby/BP_GM_lobby.ArmazenarInfoJogadores` _asbp_gm_lobby))

(event `SairSessao`
  ;[1 0.3303 0.2904] Evento para sair da sessão atual e voltar para o menu principal
  (`DestroySessionCallbackProxy.DestroySession` self
    (:`OnSuccess`
      (`GameplayStatics.OpenLevel` "LVL_menuPrincipal"))))

(event `SR_PodeIniciarPartida`
  (params (iniciarPartida :type Boolean))
  ;[1 1 1] Habilita / Desabilita o botão de iniciar a partida de acordo com o "pronto" dos jogadores
  (`Widget.SetIsEnabled` (`/Game/Interface/Lobby/WB_lobby.bt_iniciarPartida` (`self.ref_wb_lobby`)) iniciarPartida))

(fn `UserConstructionScript`)