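; Player controller for the main menu that shows the menu interface and handles going back to it.
; On BeginPlay it creates the WB_menuPrincipal widget if no valid reference exists, adds it to the viewport and sets Game and UI input mode focused on it.
; Pressing Escape calls VoltarParaMenu on that widget to return to the main menu screen.
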(event `self.ReceiveBeginPlay`
  ;[1 1 1] Adiciona a interface do menu principal a tela
  (`/Engine/EditorBlueprintResources/StandardMacros.IsValid` (`self.ref_wb_menuPrincipal`) ; verifica se o widget já foi criado
    (:`Is Valid`
      _)
    (:`Is Not Valid`
      (bind _returnvalue (`|CreateWidget` "/Game/Interface/MenuPrincipal/WB_menuPrincipal.WB_menuPrincipal_C" self)) ; cria a interface do menu
      (bind _output_get (set `self.ref_wb_menuPrincipal` _returnvalue))))
  (`UserWidget.AddToViewport` _output_get 0) ; adiciona a interface a tela
  (`WidgetBlueprintLibrary.SetInputMode_GameAndUIEx` self (`self.ref_wb_menuPrincipal`) "DoNotLock" false))

(event `Key|Escape`
  (params (Key :type "Key Structure"))
  ;[1 1 1] Tecla para voltar para o menu principal
  (:`Pressed`
    (`/Game/Interface/MenuPrincipal/WB_menuPrincipal.VoltarParaMenu` (`self.ref_wb_menuPrincipal`))))

(fn `UserConstructionScript`)