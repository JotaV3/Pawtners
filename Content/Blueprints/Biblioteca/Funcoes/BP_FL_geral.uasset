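; General Blueprint function library for respawning players and reading saved player info.
; RenascerJogador destroys the controlled pawn, unpossesses the controller and restarts it through the given GameMode at the PlayerStart looked up by player ID.
; It then points the controller's view target at that PlayerStart, not the new pawn, and returns the start.
; InfoJogador returns the SgInfoJogador field from saved data requested through a GameInstance message.
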(fn `InfoJogador`
  (returns (infoJogador :type "/Game/Geral/ST_infoJogador Structure"))
  (bind _dadossalvos (message `/Game/Geral/BPI_salvarJogo.PegarDadosSalvos` (`GameplayStatics.GetGameInstance` null)))
  (return (`/Game/Geral/BP_SG_geral.sg_infoJogador` _dadossalvos)))

(fn `Renascer Jogador`
  (params (Target :type "GameModeBase Object Reference") (controleJogador :type "PlayerController Object Reference") (IDJogador :type Integer))
  (returns (ReturnValue :type "Actor Object Reference"))
  (locals (local_gameMode :type "GameModeBase Object Reference") (controlerJogador :type "PlayerController Object Reference"))
  (bind _controlerjogador (`local.controlerJogador`))
  (bind _returnvalue (`GameModeBase.K2_FindPlayerStart` (`local.local_gameMode`) _controlerjogador (`KismetStringLibrary.Conv_IntToString` IDJogador)))
  (set `local.local_gameMode` Target)
  (bind _output_get (set `local.controlerJogador` controleJogador))
  (bind _returnvalue_2 (`Controller.K2_GetPawn` _output_get))
  (`/Engine/EditorBlueprintResources/StandardMacros.IsValid` _returnvalue_2
    (:`Is Valid`
      (`Actor.K2_DestroyActor` _returnvalue_2))
    (:`Is Not Valid`
      _))
  (`Controller.UnPossess` _controlerjogador)
  (`GameModeBase.RestartPlayerAtPlayerStart` (`local.local_gameMode`) _controlerjogador _returnvalue)
  (`PlayerController.SetViewTargetWithBlend` (`local.controlerJogador`) _returnvalue 0.0 "VTBlend_Linear" 0.0 false)
  (return _returnvalue))