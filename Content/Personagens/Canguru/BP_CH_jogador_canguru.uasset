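; Kangaroo player character with camera-relative movement, mouse-look, jumping and a name tag above the player.
; On BeginPlay the locally controlled instance passes its player info to EnviarInfoServidor, which stores it in InfoJogador.
; OnRep_infoJogador then writes the player name into the WB_etiquetaNome widget, retrying on a short timer until that widget is valid.
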(event `self.ReceiveBeginPlay`
  ;[1 1 1] Adicionar uma etiqueta de jogador para os jogadores
  (if (`self.IsLocallyControlled`)
    (bind _infojogador (`/Game/Blueprints/Biblioteca/Funcoes/BP_FL_geral.InfoJogador`))
    (`self.EnviarInfoServidor` _infojogador)))

(event `EnviarInfoServidor`
  (params (infoJogador :type "/Game/Geral/ST_infoJogador Structure"))
  ;[1 1 1] Adicionar uma etiqueta de jogador para os jogadores
  (set `self.infoJogador` infoJogador))

(event `InputAxis|MoverFrente`
  (params (AxisValue :type "Float (single-precision)"))
  ;[1 1 1] Movimentação
  (`self.AddMovementInput` (`KismetMathLibrary.GetForwardVector` (`KismetMathLibrary.MakeRotator` 0.0 0.0 (.yaw (`self.GetControlRotation`)))) AxisValue))

(event `InputAxis|MoverLado`
  (params (AxisValue :type "Float (single-precision)"))
  ;[1 1 1] Movimentação
  (`self.AddMovementInput` (`KismetMathLibrary.GetRightVector` (`KismetMathLibrary.MakeRotator` 0.0 0.0 (.yaw (`self.GetControlRotation`)))) AxisValue))

(event `InputAxis|Virar`
  (params (AxisValue :type "Float (single-precision)"))
  ;[1 1 1] Camera
  (`self.AddControllerYawInput` AxisValue))

(event `InputAction|pular`
  (params (Key :type "Key Structure"))
  ;[1 1 1] Pulo
  (:`Pressed`
    (`self.Jump`))
  (:`Released`
    (`self.StopJumping`)))

(event `InputAxis|OlharCima`
  (params (AxisValue :type "Float (single-precision)"))
  ;[1 1 1] Camera
  (`self.AddControllerPitchInput` AxisValue))

(fn `OnRep_infoJogador`
  (bind _infojogador_nomejogador (break `/Game/Geral/ST_infoJogador` (`self.infoJogador`)))
  (bind _returnvalue (`WidgetComponent.GetWidget` (`self.Widget`)))
  (`/Engine/EditorBlueprintResources/StandardMacros.IsValid` _returnvalue
    (:`Is Valid`
      ;[1 1 1] Chama a WB_etiqueta jogador e atualiza o nome do jogador para ser criado uma etiqueta com o nome dele
      (bind _aswb_etiqueta_nome (cast `/Game/Personagens/WB_etiquetaNome` _returnvalue))
      (set `/Game/Personagens/WB_etiquetaNome.nomeJogador` _infojogador_nomejogador _aswb_etiqueta_nome)
      (`/Game/Personagens/WB_etiquetaNome.NomearJogador` _aswb_etiqueta_nome))
    (:`Is Not Valid`
      ;[1 1 1] Se o widget não tiver sido criado ainda, será chamado novamente a função
      (`KismetSystemLibrary.K2_SetTimer` self "OnRep_infoJogador" 0.1))))

(fn `UserConstructionScript`)