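; BP_CH_jogador is the multiplayer player character, with movement, camera, jump and temporary air-control reduction as a stun.
; It sends player info and checkpoint transforms to the server, and OnRep fills the name tag, retrying until its widget exists.
; Mesh changes look up matching AnimBPs and rebuild an outline mesh.
; Bear-trap escape uses E presses against a timer-decayed bar, while Tick jiggles movement with sweeps so obstacles hit idle players.
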(event `PegaDados`
  ;[1 0.9442 0.1824] Muda mesh e envia a info
  (if (`self.IsLocallyControlled`)
    (`self.InicializarCheckpoint`)
    (bind _infojogador (`/Game/Blueprints/Biblioteca/Funcoes/BP_FL_geral.InfoJogador`))
    (bind (_nomejogador _imagempersonagemjogador _personagemjogador _statusjogador) (break `/Game/Geral/ST_infoJogador` _infojogador))
    ;;[1 1 1] Envia as informações do jogador para o servidor
    (bind _output_get (set `self.infoJogador` (make `/Game/Geral/ST_infoJogador` _nomejogador _imagempersonagemjogador _personagemjogador _statusjogador (stale `PegaMesh` _skel_mesh))))
    (`self.SE_EnviarInfo` _output_get)))

(event `PegaMesh`
  (params (in_CharStruct :type "/Game/Interface/MenuPrincipal/Paginas/CharacterStruct Structure"))
  ;[1 0.9442 0.1824] Muda mesh e envia a info
  (bind _skel_mesh (`self.MudaTudoCharacter` in_CharStruct)))

(event `CustomEvent`
  (params (infoJogador :type "/Game/Geral/ST_infoJogador Structure"))
  ;[1 0.9442 0.1824] Muda mesh e envia a info
  ;;[1 1 1] Envia as informações do jogador para o servidor
  (set `self.infoJogador` infoJogador))

(event `self.ReceiveTick`
  (params (DeltaSeconds :type "Float (single-precision)"))
  (bind _returnvalue (`self.K2_GetActorRotation`))
  (bind _charactermovement (`self.CharacterMovement`))
  ;[1 1 1] Resolve o problema do obstaculo atravessar o personagem caso o mesmo esteja parado
  (`MovementComponent.K2_MoveUpdatedComponent` _charactermovement (0.1 0.1 0.0) _returnvalue true false)
  (`MovementComponent.K2_MoveUpdatedComponent` _charactermovement (-0.1 -0.1 0.0) _returnvalue true false))

(event `self.ReceiveBeginPlay`
  (if (`self.IsLocallyControlled`)
    (`self.InicializarCheckpoint`)
    (bind _infojogador (`/Game/Blueprints/Biblioteca/Funcoes/BP_FL_geral.InfoJogador`))
    ;[1 1 1] Envia as informações do jogador para o servidor
    (`self.SE_EnviarInfo` _infojogador)))

(event `LiberarPressionamentoTecla`
  (params (widget :type "/Game/Blueprints/Jogo/Interativos/Obstaculos/ArmadilhaUrso/WB_pressionarTecla Object Reference") (liberar :type Boolean))
  ;[1 1 1] Armadilha de urso
  ;;[1 1 1] Libera a tecla de pressionamento para que o jogador escape da armadilha
  (`self.IniciarReferencias` widget liberar)
  (`Widget.SetVisibility` (`self.wb_pressionarTecla`) "Visible") ; Torna visível o widget que mostra a barra de progresso de escape da armadilha de urso
  ;;;[1 1 1] A cada x segundos é decrementado a barra de progresso de escape da armadilha
  (bind _returnvalue (`KismetSystemLibrary.K2_SetTimerDelegate` (delegate `DecrementarBarraProgresso`) (`self.tempoDecremento`) true))
  (set `self.ref_temporizador` _returnvalue))

(event `SE_EnviarInfo`
  (params (infoJogador :type "/Game/Geral/ST_infoJogador Structure"))
  ;[1 1 1] Envia as informações do jogador para o servidor
  (set `self.infoJogador` infoJogador))

(event `DecrementarBarraProgresso`
  ;[1 1 1] Armadilha de urso
  ;;[1 1 1] Libera a tecla de pressionamento para que o jogador escape da armadilha
  ;;;[1 1 1] A cada x segundos é decrementado a barra de progresso de escape da armadilha
  (`self.DecrementarPressionamento`))

(event `InputAxis|MoverFrente`
  (params (AxisValue :type "Float (single-precision)"))
  ;[1 1 1] Movimentação
  (`self.AddMovementInput` (`KismetMathLibrary.GetForwardVector` (`KismetMathLibrary.MakeRotator` 0.0 0.0 (.yaw (`self.GetControlRotation`)))) AxisValue))

(event `InicializarCheckpoint`
  ;[1 1 1] Checkpoint
  ;;[1 1 1] Inicia o checkpoint como a posição do player start no index 0
  (bind _output_get (set `self.checkpoint` (`self.GetTransform`)))
  (`self.SR_EnviarCheckpoint` _output_get))

(event `Key|E`
  (params (Key :type "Key Structure"))
  ;[1 1 1] Armadilha de urso
  ;;[1 1 1] Tecla configurada para escapar da armadilha, só é liberada quando o jogador cai na armadilha
  (:`Pressed`
    (if (`self.liberado`)
      (`self.IncrementarPressionamento`)
      (`self.SR_SoltarJogaodor`)
      ;;;[1 1 1] Desabilita o timer que decrementa o progresso da barra, desabilita a tecla de escape da armadilha e torna o widget da armadilha escondido
      (`KismetSystemLibrary.K2_ClearAndInvalidateTimerHandle` (`self.ref_temporizador`))
      (set `self.liberado` false)
      (`Widget.SetVisibility` (`self.wb_pressionarTecla`) "Hidden"))))

(event `AtualizarCheckpoint`
  ;[1 1 1] Checkpoint
  ;;[1 1 1] Atualiza/Salva o ponto de renascimento do jogador na variável chekpoint e envia para o servidor
  (bind _output_get (set `self.checkpoint` (`self.GetTransform`)))
  (`self.SR_EnviarCheckpoint` _output_get))

(event `InputAxis|MoverLado`
  (params (AxisValue :type "Float (single-precision)"))
  ;[1 1 1] Movimentação
  (`self.AddMovementInput` (`KismetMathLibrary.GetRightVector` (`KismetMathLibrary.MakeRotator` 0.0 0.0 (.yaw (`self.GetControlRotation`)))) AxisValue))

(event `SR_EnviarCheckpoint`
  (params (checkpoint :type "Transform Structure"))
  ;[1 1 1] Checkpoint
  ;;[1 1 1] Atualiza/Salva o ponto de renascimento do jogador na variável chekpoint e envia para o servidor
  (set `self.checkpoint` checkpoint))

(event `InputAxis|Virar`
  (params (AxisValue :type "Float (single-precision)"))
  ;[1 1 1] Camera
  (`self.AddControllerYawInput` AxisValue))

(event `SR_SoltarJogaodor`
  ;[1 1 1] Armadilha de urso
  ;;[1 1 1] Desprende o jogador da armadilha / reabilita os movimentos do jogador
  (`CharacterMovementComponent.SetMovementMode` (`self.CharacterMovement`) "MOVE_Walking" 0))

(event `InputAction|pular`
  (params (Key :type "Key Structure"))
  ;[1 1 1] Pulo
  (:`Pressed`
    (`self.Jump`)
    (if (not (`NavMovementComponent.IsFalling` (`self.CharacterMovement`)))
      (`GameplayStatics.PlaySound2D` "/Game/Blueprints/Jogo/Som/SW_pulo.SW_pulo" 1.0 1.0 0.0 null null)))
  (:`Released`
    (`self.StopJumping`)))

(event `InputAxis|OlharCima`
  (params (AxisValue :type "Float (single-precision)"))
  ;[1 1 1] Camera
  (`self.AddControllerPitchInput` AxisValue))

(event `SR_ControleAereo`
  ;[1 1 1] Desabilita o controle aéreo do jogador quando ele é lançado por algum motivo, simulanto um stun
  (`|ExecutionSequence`
    (:`then_0`
      (`self.DesabilitarControleAereo` self))
    (:`then_1`
      (`KismetSystemLibrary.Delay` 3.0)
      (`self.HabilitarControleAereo` self))))

(fn `ChangeMeshPlayer`
  (params (SkeletalMesh :type "SkeletalMesh Object Reference"))
  (bind (_value _returnvalue) (`BlueprintMapLibrary.Map_Find` (`self.AnimB_array`) SkeletalMesh))
  (`SkinnedMeshComponent.SetSkinnedAssetAndUpdate` (`self.Mesh`) SkeletalMesh true)
  (if _returnvalue
    (`KismetSystemLibrary.PrintString` (`KismetSystemLibrary.GetClassDisplayName` _value))
    (`SkeletalMeshComponent.SetAnimInstanceClass` (`self.Mesh`) null)
    (else
      (`KismetSystemLibrary.PrintString` (`KismetStringLibrary.Concat_StrStr` "Anim_BP_not_finded for" (`KismetSystemLibrary.GetDisplayName` SkeletalMesh))))))

(fn `CreateOutline`
  (bind _mesh (`self.Mesh`))
  (bind _outlinemesh (`self.Outlinemesh`))
  (`SkinnedMeshComponent.SetSkinnedAssetAndUpdate` _outlinemesh (`SkinnedMeshComponent.SkeletalMesh` _mesh) true)
  (`SkeletalMeshComponent.SetAnimInstanceClass` (`self.Outlinemesh`) (`SkeletalMeshComponent.AnimClass` _mesh))
  (for (_ _array_index) (`MeshComponent.GetMaterials` _outlinemesh)
    (`PrimitiveComponent.SetMaterial` _outlinemesh _array_index "/Game/Assets/Postprocess/OutlineMat.OutlineMat")))

(fn `DesabilitarControleAereo`
  (set `CharacterMovementComponent.AirControl` 0.2 (`self.CharacterMovement`)))

(fn `HabilitarControleAereo`
  (set `CharacterMovementComponent.AirControl` 0.6 (`self.CharacterMovement`)))

(fn `IniciarReferencias`
  (params (wb_pressionarTecla :type "/Game/Blueprints/Jogo/Interativos/Obstaculos/ArmadilhaUrso/WB_pressionarTecla Object Reference") (Liberar :type Boolean))
  ;[1 1 1] Inicia algumas referências
  (set `self.wb_pressionarTecla` wb_pressionarTecla)
  (set `self.liberado` Liberar) ; Precisa ser replicada para o jogador saber se está liberado ou não o input
  (bind _output_get (set `/Game/Blueprints/Jogo/Interativos/Obstaculos/ArmadilhaUrso/WB_pressionarTecla.porcentagem` 0.0 (`self.wb_pressionarTecla`)))
  (set `self.pressionamento` _output_get))

(fn `MudaTudoCharacter`
  (params (in_CharStruct :type "/Game/Interface/MenuPrincipal/Paginas/CharacterStruct Structure"))
  (returns (Skel_Mesh :type "SkeletalMesh Object Reference"))
  (bind (_out_charstruct _skeletalmesh _havedata_out) (`/Game/Blueprints/Biblioteca/Macro/CharacterMacroLibrary.Getdata_SKMesh_Macro` in_CharStruct)
    (:`exec_out`
      (bind (_value _returnvalue) (`BlueprintMapLibrary.Map_Find` (`self.AnimB_array`) _skeletalmesh))
      (if _returnvalue
        (bind _out_charstruct_2 (`/Game/Blueprints/Biblioteca/Macro/CharacterMacroLibrary.Change_SKMesh_Macro` _out_charstruct _havedata_out _value)
          (:`exec_out`
            (`self.CreateOutline`)
            (bind (_name _icone _skel_mesh) (break `/Game/Interface/MenuPrincipal/Paginas/CharacterStruct` _out_charstruct_2))
            (set `self.Skel Mesh` _skel_mesh)
            (return _skel_mesh)))
        (else
          (`KismetSystemLibrary.PrintString` (`KismetStringLibrary.Concat_StrStr` "AnimBp not found for " (`KismetSystemLibrary.GetDisplayName` _skeletalmesh))))))))

(fn `OnRep_infoJogador`
  (bind _infojogador_nomejogador (break `/Game/Geral/ST_infoJogador` (`self.infoJogador`)))
  (bind _returnvalue (`WidgetComponent.GetWidget` (`self.Widget`)))
  (`/Engine/EditorBlueprintResources/StandardMacros.IsValid` _returnvalue
    (:`Is Valid`
      ;[1 1 1] Chama a WB_etiqueta jogador e atualiza o nome do jogador para ser criado uma etiqueta com o nome dele
      (bind _aswb_etiqueta_nome (cast `/Game/Personagens/WB_etiquetaNome` _returnvalue))
      (set `/Game/Personagens/WB_etiquetaNome.nomeJogador` _infojogador_nomejogador _aswb_etiqueta_nome)
      (`/Game/Personagens/WB_etiquetaNome.NomearJogador` _aswb_etiqueta_nome))
    (:`Is Not Valid`
      ;[1 1 1] Se o widget não tiver sido criado ainda, será chamado novamente a função
      (`KismetSystemLibrary.K2_SetTimer` self "OnRep_infoJogador" 0.1))))

(fn `UserConstructionScript`)